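; Actor component that plays branching VR dialogue with subtitles, sound and body/face montages, using the owner's BP_VR_HUD_Actor widgets.
; Each entry runs subtitles and sounds in parallel, with montages advancing on SoundFinished and subtitles also mirrored to listed players.
; When sounds end, it shows pooled answer buttons or advances; a picked answer plays as a temporary dialogue, then jumps by name.
; Attached and positional sounds go through server-to-multicast events; 2D sound stays local.
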(event `Answer Selected_Event_0`
  (params (`Answer Index` :type Integer))
  (bind _returnvalue (`self.GetOwner`))
  (bind (_answertitle _subtitles _sound _dialoguetogo _actor_locationdata) (break `/Game/VRSubtitle/Structures/F_AnswerStructure` (`|GetArrayItem` (`.Answers_18_B26CFB4645DA00B03C1B5683541276E4` (break `/Game/VRSubtitle/Structures/F_AdvancedDialogueStructure` (`|GetArrayItem` (`self.All Dialogues`) (`self.Dialogue Index`)))) `Answer Index`)))
  ;[1 1 1] On Answer Selected
  (set `self.Came From Answer?` true) ; I used the same codes for answers and normal dialogues. \nI use this boolean to distinguish between the two.
  (bind _output_get (set `self.Answer Dialogue` (`|MakeArray` (make `/Game/VRSubtitle/Structures/F_AdvancedDialogueStructure` _subtitles _sound _dialoguetogo _actor_locationdata) :!type "/Game/VRSubtitle/Structures/F_AdvancedDialogueStructure Structure"))) ; Saving the dialogue that should start
  (set `self.WarpPointName` (`KismetTextLibrary.Conv_TextToString` _answertitle))
  (`self.Reset All Indexes`) ; Resetting all indexes (Dialogue index, Sound index etc)
  (`self.Start A Dialouge` _output_get (`self.Show Subtitles To These Players`)) ; Starting the Answer
  (for _array_element (`self.AnswerWidgets`)
    (`Widget.RemoveFromParent` _array_element))
  (if (`KismetSystemLibrary.DoesImplementInterface` _returnvalue "/Game/VRSubtitle/Blueprints/BI_VR_Dialogue_Interface.BI_VR_Dialogue_Interface_C")
    (message `/Game/VRSubtitle/Blueprints/BI_VR_Dialogue_Interface.Start Waiting For Answer` _returnvalue false)))

(event `self.ReceiveBeginPlay`
  ;[1 1 1] Seting the widgets
  (bind (_asbp_vrhudactor _success) (`self.Get VR Hud Actor`))
  (if _success
    (bind _aswbp_subtitle (cast `/Game/VRSubtitle/Widgets/WBP_Subtitle` (`WidgetComponent.GetUserWidgetObject` (`/Game/VRSubtitle/Blueprints/BP_VR_HUD_Actor.3DWidget` _asbp_vrhudactor))))
    (bind _output_get (set `self.DialogueWidgetRef` _aswbp_subtitle)) ; Save the reference of the SubtitleWidget
    (bind _subtitletext (`/Game/VRSubtitle/Widgets/WBP_Subtitle.SubtitleText` _output_get))
    (`TextBlock.SetText` _subtitletext "")
    (bind _output_get_2 (set `self.Subtitle Text Ref` _subtitletext)) ; Save the reference of the subtitle text
    (`ScaleBox.SetUserSpecifiedScale` (`/Game/VRSubtitle/Widgets/WBP_Subtitle.ScaleBox_0` _output_get) (`self.Subtitle Scale`)) ; Seting Subtitle Scale
    (`Widget.SetRenderOpacity` _output_get_2 (`KismetMathLibrary.SelectFloat` 1.0 0.0 (`self.Subtitles On?`))) ; Setting visiblity of subtitle according the "Subtitle On?" bool
    (bind _3d_answerswidget (`/Game/VRSubtitle/Blueprints/BP_VR_HUD_Actor.3D_AnswersWidget` _asbp_vrhudactor))
    (bind _aswbp_answers (cast `/Game/VRSubtitle/Widgets/WBP_Answers` (`WidgetComponent.GetUserWidgetObject` _3d_answerswidget)))
    (set `self.3D Answers Widget` _3d_answerswidget)
    (set `self.AnswersBox` (`/Game/VRSubtitle/Widgets/WBP_Answers.AnswersBox` _aswbp_answers))
    ;;[1 1 1] For Loop
    (for _ (range 9)
      (bind _returnvalue (`|CreateWidget` "/Game/VRSubtitle/Widgets/WBP_AnAnswerWidget.WBP_AnAnswerWidget_C"))
      (`ScaleBox.SetUserSpecifiedScale` (`/Game/VRSubtitle/Widgets/WBP_AnAnswerWidget.ScaleBox_1` _returnvalue) (`self.Answer Scale`)) ; Setting Answer Scale
      (bind _returnvalue_2 (`KismetArrayLibrary.Array_Add` (`self.AnswerWidgets`) _returnvalue))
      (set `/Game/VRSubtitle/Widgets/WBP_AnAnswerWidget.Answer Index` _returnvalue_2 _returnvalue) ; Sending their indexes to Answers Buttons
      (add `/Game/VRSubtitle/Widgets/WBP_AnAnswerWidget.Answer Selected` _returnvalue (delegate `Answer Selected_Event_0`)) ; Binding "AnswerSelected" event dispatchers to an event
    )
    (else
      (`self.Show Error Message` "Please Add BP_VR_HUD_Actor to your Pawn / Character"))))

(event `Next Subtitle`
  (bind _subtitle_index (`self.Subtitle Index`))
  (bind ((`Subtitles_3_45F961724E75F683443E4FBA6089B0A2` _subtitles) (`Sounds_6_EEBA3BED45B8FA6D22886DA8F06143D3` _sounds) (`DialogueName_10_D8535BE44B192A8A2AD0ADA129EE3924` _dialoguename)) (break `/Game/VRSubtitle/Structures/F_AdvancedDialogueStructure` (`|GetArrayItem` (`self.All Dialogues`) (`self.Dialogue Index`))))
  (bind (_subtitle _duration) (break `/Game/VRSubtitle/Structures/F_Subtitle` (`|GetArrayItem` _subtitles _subtitle_index)))
  ;[1 1 1] Subtitle
  (remove `self.Sound Finished` (delegate `Next Subtitle`))
  (`/Engine/EditorBlueprintResources/StandardMacros.IncrementInt` (`self.Subtitle Index`) :!label _label
    (:`  `
      (`self.Text Finished`)
      (if (`KismetArrayLibrary.Array_IsValidIndex` _subtitles _subtitle_index) :!label _label_2
        (`self.Show Subtitle` _subtitle (`self.Show Subtitles To These Players`)) ; Shows subtitles to  "Show Subtitles To These Players"
        (bind _subtitle_text_ref (`self.Subtitle Text Ref`)
          (:`then`
            (`TextBlock.SetText` _subtitle_text_ref _subtitle) ; Shows subtitles to owner
            (if (!= _duration 0.0)
              (`KismetSystemLibrary.Delay` _duration)
              (goto _label)
              (else
                (add `self.Sound Finished` (delegate `Next Subtitle`)))))
          (:`else`))
        (else
          (set `self.Subtitle Index` 0))))))

(event `Show Subtitle`
  (params (Text :type Text) (`Players To Show Subtitle` :type "Array of Actor Object Reference"))
  ;[1 1 1] Subtitle
  (for _array_element `Players To Show Subtitle`
    (bind _returnvalue (`Actor.GetComponentByClass` _array_element "BP_AdvancedDialogueComponent_C"))
    (`/Engine/EditorBlueprintResources/StandardMacros.IsValid` _returnvalue
      (:`Is Valid`
        (`self.Set Subtitle` _returnvalue Text)))))

(event `Start A Dialouge`
  (params (`Advanced Dialogue` :type "Array of /Game/VRSubtitle/Structures/F_AdvancedDialogueStructure Structure") (`Show Subtitles to These Players` :type "Array of Actor Object Reference"))
  (bind _sound_index (`self.Sound Index`))
  (bind ((`Subtitles_3_45F961724E75F683443E4FBA6089B0A2` _subtitles) (`Sounds_6_EEBA3BED45B8FA6D22886DA8F06143D3` _sounds) (`DialogueName_10_D8535BE44B192A8A2AD0ADA129EE3924` _dialoguename)) (break `/Game/VRSubtitle/Structures/F_AdvancedDialogueStructure` (`|GetArrayItem` (`self.All Dialogues`) (`self.Dialogue Index`))))
  (bind ((`DialogueName_10_D8535BE44B192A8A2AD0ADA129EE3924` _dialoguename_2) (`Actor-LocationData_13_9143C2534F14DA822F0035B7B5B22A8B` _actor_locationdata)) (break `/Game/VRSubtitle/Structures/F_AdvancedDialogueStructure` (`|GetArrayItem` (`self.All Dialogues`) (`self.Dialogue Index`))))
  (bind ((`ActortoAffect_2_BBB526274587A0935E9B6A87D4220AEF` _actortoaffect) (`Location_5_C2D4BBBB4B01F6949619C198BB2A6F3C` _location)) (break `/Game/VRSubtitle/Structures/F_ActorToAffect` _actor_locationdata))
  (bind (_sound _afterdelay _volume) (break `/Game/VRSubtitle/Structures/F_Sound` (`|GetArrayItem` _sounds _sound_index)))
  (bind _output_get (set `self.All Dialogues` `Advanced Dialogue`)) ; Saving the All dialogues (I used the same codes for answers and normal dialogues.\nSo this variable can sometimes contain only the answers)
  (if (not (`self.Came From Answer?`))
    (set `self.All Dialogues GRAND` _output_get))
  ;[1 1 1] Saving the "Show Subtitles to These Players" variable if is valid.
  (if (`KismetArrayLibrary.Array_IsValidIndex` `Show Subtitles to These Players`)
    (`/Engine/EditorBlueprintResources/StandardMacros.IsValid` (`|GetArrayItem` `Show Subtitles to These Players`)
      (:`Is Valid`
        (set `self.Show Subtitles To These Players` `Show Subtitles to These Players`))
      (:`Is Not Valid`
        _)))
  (`self.Dialogue Started` _dialoguename)
  (`|ExecutionSequence`
    (:`then_0`
      (goto _label_2))
    (:`then_1`
      ;[1 1 1] Sound
      (if (`KismetArrayLibrary.Array_IsValidIndex` _sounds _sound_index) :!label _label_3
        (if (`KismetSystemLibrary.IsValidSoftObjectReference` _sound)
          (`self.Sound Started` _dialoguename_2)
          (`self.Unbind Montage Events`)
          (bind _returnvalue (`KismetSystemLibrary.LoadAsset_Blocking` _sound))
          (`/Engine/EditorBlueprintResources/StandardMacros.IsValid` _actortoaffect
            (:`Is Valid`
              (bind _assound_wave (cast `SoundWave` _returnvalue :!pure true))
              (`self.Spawn Sound Attached_Server` _assound_wave (`Actor.RootComponent` _actortoaffect) _volume)
              (bind _returnvalue_2 (+ (`SoundBase.Duration` _assound_wave) _afterdelay))
              (`KismetSystemLibrary.Delay` _returnvalue_2))
            (:`Is Not Valid`
              (if (== _location (0.0 0.0 0.0) :`ErrorTolerance` 1.0)
                ;;[1 1 1] NOT REPLICATED
                (bind _returnvalue_3 (`GameplayStatics.SpawnSound2D` _assound_wave _volume 1.0 0.0 null))
                (set `self.Sound` _returnvalue_3)
                (`KismetSystemLibrary.Delay` _returnvalue_2)
                (else
                  (`self.Spawn Sound 3D_Server` _assound_wave _location _volume)
                  (`KismetSystemLibrary.Delay` _returnvalue_2)))))
          (else
            (`KismetSystemLibrary.Delay` _afterdelay)))
        (`/Engine/EditorBlueprintResources/StandardMacros.IncrementInt` (`self.Sound Index`)
          (:`  `
            (`self.Sound Finished`)
            (goto _label_3)))
        (else
          (set `self.Sound Index` 0)
          (`self.Start Answers`))))
    (:`then_2`
      (`self.Play Body Montage`))
    (:`then_3`
      (`self.Play Face Montage`))))

(event `Set Subtitle`
  (params (Text :type Text))
  ;[1 1 1] Subtitle
  (bind _subtitle_text_ref (`self.Subtitle Text Ref`)
    (:`then`
      (`TextBlock.SetText` _subtitle_text_ref Text))
    (:`else`)))

(event `Set Subtitles On/Off`
  (params (`Subtitles On?` :type Boolean))
  ;[1 1 1] Subtitle
  (set `self.Subtitles On?` `Subtitles On?`))

(event `Remove Subtitle`
  (params (`Players To Show Subtitle` :type "Array of Actor Object Reference (by ref)"))
  ;[1 1 1] Subtitle
  (`self.Show Subtitle` "" `Players To Show Subtitle`))

(event `Spawn Sound Attached_Server`
  (params (Sound :type "SoundBase Object Reference") (AttachToComponent :type "SceneComponent Object Reference") (VolumeMultiplier :type "Float (double-precision)"))
  ;[1 1 1] Sound
  (`self.Spawn Sound Attached_Multicast` Sound AttachToComponent VolumeMultiplier))

(event `Spawn Sound Attached_Multicast`
  (params (Sound :type "SoundBase Object Reference") (AttachToComponent :type "SceneComponent Object Reference") (VolumeMultiplier :type "Float (double-precision)"))
  ;[1 1 1] Sound
  (bind _returnvalue (`GameplayStatics.SpawnSoundAttached` Sound AttachToComponent "None" (0.0 0.0 0.0) (struct) "SnapToTarget" false VolumeMultiplier 1.0 0.0 (`self.Attenuation Settings`) null))
  (set `self.Sound` _returnvalue))

(event `Spawn Sound 3D_ Multicast`
  (params (Sound :type "SoundBase Object Reference") (Location :type "Vector Structure") (VolumeMultiplier :type "Float (double-precision)"))
  ;[1 1 1] Sound
  (bind _returnvalue (`GameplayStatics.SpawnSoundAtLocation` Sound Location (struct) VolumeMultiplier 1.0 0.0 (`self.Attenuation Settings`) null))
  (set `self.Sound` _returnvalue))

(event `Spawn Sound 3D_Server`
  (params (Sound :type "SoundBase Object Reference") (Location :type "Vector Structure") (VolumeMultiplier :type "Float (double-precision)"))
  ;[1 1 1] Sound
  (`self.Spawn Sound 3D_ Multicast` Sound Location VolumeMultiplier))

(event `Play Body Montage`
  (bind _body_montage_index (`self.Body Montage Index`))
  (bind ((`ActortoAffect_2_BBB526274587A0935E9B6A87D4220AEF` _actortoaffect) (`BodyMontage_9_644C726543D44140D2976C8F25512AA3` _bodymontage)) (break `/Game/VRSubtitle/Structures/F_ActorToAffect` (`.Actor-LocationData_13_9143C2534F14DA822F0035B7B5B22A8B` (break `/Game/VRSubtitle/Structures/F_AdvancedDialogueStructure` (`|GetArrayItem` (`self.All Dialogues`) (`self.Dialogue Index`))))))
  (bind _animmontage (break `/Game/VRSubtitle/Structures/F_AnimMontage` (`|GetArrayItem` _bodymontage _body_montage_index)))
  ;[1 1 1] Body Anim Montage
  (`/Engine/EditorBlueprintResources/StandardMacros.IsValid` _actortoaffect :!label _label_4
    (:`Is Valid`
      (if (`KismetArrayLibrary.Array_IsValidIndex` _bodymontage _body_montage_index)
        (if (`KismetSystemLibrary.DoesImplementInterface` _actortoaffect "/Game/VRSubtitle/Blueprints/BI_AdvancedDialogue.BI_AdvancedDialogue_C")
          (if (`KismetSystemLibrary.IsValidSoftObjectReference` _animmontage)
            (message `/Game/VRSubtitle/Blueprints/BI_AdvancedDialogue.Play Body Montage` _actortoaffect _animmontage)
            (if (`KismetArrayLibrary.Array_IsValidIndex` _bodymontage (+ (`self.Body Montage Index`) 1))
              (add `self.Sound Finished` (delegate `Next Body Montage`))
              (else
                (remove `self.Sound Finished` (delegate `Next Body Montage`))))
            (else
              (set `self.Body Montage Index` 0 :!label _label_5)
              (`self.Body Montages Finished`)))
          (else
            (`self.Show Error Message` "ERROR: Advanced Dialogue -> The Pawn has not BPI_AdvancedDialogue blueprint interface")
            (goto _label_5)))
        (else
          (goto _label_5))))
    (:`Is Not Valid`
      (goto _label_5))))

(event `Next Body Montage`
  ;[1 1 1] Body Anim Montage
  (remove `self.Sound Finished` (delegate `Next Body Montage`))
  (`/Engine/EditorBlueprintResources/StandardMacros.IncrementInt` (`self.Body Montage Index`)
    (:`  `
      (goto _label_4))))

(event `Unbind Montage Events`
  (remove `self.Sound Finished` (delegate `Next Face Montage`))
  (remove `self.Sound Finished` (delegate `Next Body Montage`)))

(event `Play Face Montage`
  (bind _face_montage_index (`self.Face Montage Index`))
  (bind ((`ActortoAffect_2_BBB526274587A0935E9B6A87D4220AEF` _actortoaffect) (`FaceMontage_11_DE7AFCEE4DC4B58A0CDD17B5D2C0B76D` _facemontage)) (break `/Game/VRSubtitle/Structures/F_ActorToAffect` (`.Actor-LocationData_13_9143C2534F14DA822F0035B7B5B22A8B` (break `/Game/VRSubtitle/Structures/F_AdvancedDialogueStructure` (`|GetArrayItem` (`self.All Dialogues`) (`self.Dialogue Index`))))))
  (bind _animmontage (break `/Game/VRSubtitle/Structures/F_AnimMontage` (`|GetArrayItem` _facemontage _face_montage_index)))
  ;[1 1 1] Face Anim Montage
  (`/Engine/EditorBlueprintResources/StandardMacros.IsValid` _actortoaffect :!label _label_6
    (:`Is Valid`
      (if (`KismetArrayLibrary.Array_IsValidIndex` _facemontage _face_montage_index)
        (if (`KismetSystemLibrary.DoesImplementInterface` _actortoaffect "/Game/VRSubtitle/Blueprints/BI_AdvancedDialogue.BI_AdvancedDialogue_C")
          (if (`KismetSystemLibrary.IsValidSoftObjectReference` _animmontage)
            (message `/Game/VRSubtitle/Blueprints/BI_AdvancedDialogue.Play Face Montage` _actortoaffect _animmontage)
            (if (`KismetArrayLibrary.Array_IsValidIndex` _facemontage (`self.Face Montage Index`))
              (add `self.Sound Finished` (delegate `Next Face Montage`))
              (else
                (remove `self.Sound Finished` (delegate `Next Face Montage`))))
            (else
              (set `self.Face Montage Index` 0 :!label _label_7)
              (`self.Face Montages Finished`)))
          (else
            (`self.Show Error Message` "ERROR: Advanced Dialogue -> The Pawn has not BPI_AdvancedDialogue blueprint interface")
            (goto _label_7)))
        (else
          (goto _label_7))))
    (:`Is Not Valid`
      (goto _label_7))))

(event `Next Face Montage`
  ;[1 1 1] Face Anim Montage
  (remove `self.Sound Finished` (delegate `Next Face Montage`))
  (`/Engine/EditorBlueprintResources/StandardMacros.IncrementInt` (`self.Face Montage Index`)
    (:`  `
      (goto _label_6))))

(event `Start Answers`
  (bind _returnvalue (`self.GetOwner`))
  (bind _dialogue_index (`self.Dialogue Index`))
  (bind _all_dialogues (`self.All Dialogues`))
  (bind ((`Answers_18_B26CFB4645DA00B03C1B5683541276E4` _answers)) (break `/Game/VRSubtitle/Structures/F_AdvancedDialogueStructure` (`|GetArrayItem` (`self.All Dialogues`) (`self.Dialogue Index`))))
  (bind ((`DialogueName_10_D8535BE44B192A8A2AD0ADA129EE3924` _dialoguename) (`NextAcceptable?_23_A10336994623226C14A5DEBD594C1BA5` _nextacceptable_) (`DialoguetoGo_26_1A10C81E47417668B4632A9138D774C3` _dialoguetogo)) (break `/Game/VRSubtitle/Structures/F_AdvancedDialogueStructure` (`|GetArrayItem` _all_dialogues (- _dialogue_index 1))))
  ;[1 1 1] Answers
  (if (`self.Came From Answer?`)
    ;;[1 1 1] Came from answer
    (bind (_index _success_) (`self.Find Dialogue To Go` (`.DialogueName_10_D8535BE44B192A8A2AD0ADA129EE3924` (break `/Game/VRSubtitle/Structures/F_AdvancedDialogueStructure` (`|GetArrayItem` (`self.All Dialogues`))))))
    (if _success_
      (set `self.Dialogue Index` _index)
      (set `self.Came From Answer?` false)
      (`self.Start A Dialouge` (`self.All Dialogues GRAND`) (`self.Show Subtitles To These Players`))
      (else
        (`self.Show Error Message` "ERROR: AdvancedDialogueSystem -> Dialogue to Go value is not same with the Dialogue Names")))
    (elif (`KismetArrayLibrary.Array_IsValidIndex` _answers)
      (set `self.All Dialogues GRAND` (`self.All Dialogues`)) ; We save it for later use.
      (bind _subtitle_text_ref (`self.Subtitle Text Ref`)
        (:`then`
          (`TextBlock.SetText` _subtitle_text_ref ""))
        (:`else`
          _))
      (`self.Remove Subtitle` (`self.Show Subtitles To These Players`))
      (if (`KismetArrayLibrary.Array_IsValidIndex` (`self.AnswerWidgets`))
        (if (`KismetSystemLibrary.DoesImplementInterface` _returnvalue "/Game/VRSubtitle/Blueprints/BI_VR_Dialogue_Interface.BI_VR_Dialogue_Interface_C")
          (message `/Game/VRSubtitle/Blueprints/BI_VR_Dialogue_Interface.Start Waiting For Answer` _returnvalue true)
          ;;[1 1 1] We display the answers on the "AnswersBox".
          (bind _answersbox (`self.AnswersBox` :!label _label_8)
            (:`then`
              (for (_array_element _array_index) _answers
                (bind _output (`|GetArrayItem` (`self.AnswerWidgets`) _array_index))
                (`TextBlock.SetText` (`/Game/VRSubtitle/Widgets/WBP_AnAnswerWidget.AnswerText` _output) (`.AnswerTitle_3_16851E884EDF01D643D0899005578478` (break `/Game/VRSubtitle/Structures/F_AnswerStructure` _array_element)))
                (`PanelWidget.AddChild` _answersbox _output)
                (`UserWidget.SetPadding` _output (make `Margin` 10.0 10.0 10.0 10.0))))
            (:`else`)))
        (else
          (goto _label_8)))
      (else
        (bind _result (`/Engine/EditorBlueprintResources/StandardMacros.IncrementInt` _dialogue_index)
          (:`  `
            (if (`KismetArrayLibrary.Array_IsValidIndex` _all_dialogues _result)
              (if _nextacceptable_
                (`self.Dialogue Finished` _dialoguename)
                (`self.Start A Dialouge` (`self.All Dialogues`) (`self.Show Subtitles To These Players`))
                (elif (`KismetStringLibrary.NotEqual_StrStr` _dialoguetogo)
                  (bind (_index_2 _success__2) (`self.Find Dialogue To Go` _dialoguetogo))
                  (if _success__2
                    (set `self.Dialogue Index` _index_2)
                    (set `self.Came From Answer?` false)
                    (`self.Start A Dialouge` (`self.All Dialogues GRAND`) (`self.Show Subtitles To These Players`))
                    (else
                      (`self.Dialogue Finished` _dialoguename :!label _label_9)
                      (`self.All Dialogues Finished`)
                      (bind _subtitle_text_ref_2 (`self.Subtitle Text Ref`)
                        (:`then`
                          (`TextBlock.SetText` _subtitle_text_ref_2 ""))
                        (:`else`
                          _))
                      (`self.Reset All Indexes`)
                      (`self.Remove Subtitle` (`self.Show Subtitles To These Players`))))
                  (else
                    (goto _label_9))))
              (else
                (goto _label_9)))))))))

(fn `Find Dialogue To Go`
  (params (`Item to Find` :type String))
  (returns (Index :type Integer) (`Success?` :type Boolean))
  (for (_array_element _array_index) (`self.All Dialogues GRAND`)
    (if (`KismetStringLibrary.EqualEqual_StrStr` (`.DialogueName_10_D8535BE44B192A8A2AD0ADA129EE3924` (break `/Game/VRSubtitle/Structures/F_AdvancedDialogueStructure` _array_element)) `Item to Find`)
      (return _array_index true)))
  (return 0 false))

(fn `Get VR Hud Actor`
  (returns (`AsBP VRHUDActor` :type "/Game/VRSubtitle/Blueprints/BP_VR_HUD_Actor Object Reference") (Success :type Boolean))
  (for _array_element (`Actor.K2_GetComponentsByClass` (`self.GetOwner`) "/Script/Engine.ChildActorComponent")
    (bind _asbp_vr_hud_actor (cast `/Game/VRSubtitle/Blueprints/BP_VR_HUD_Actor` (`ChildActorComponent.ChildActor` _array_element)))
    (return _asbp_vr_hud_actor true))
  (return null false))

(fn `OnRep_Subtitles On?`
  (bind _subtitle_text_ref (`self.Subtitle Text Ref`)
    (:`then`
      (`Widget.SetRenderOpacity` _subtitle_text_ref (`KismetMathLibrary.SelectFloat` 1.0 0.0 (`self.Subtitles On?`))))
    (:`else`
      _))
  (return))

(fn `Reset All Indexes`
  (set `self.Dialogue Index` 0)
  (set `self.Subtitle Index` 0)
  (set `self.Body Montage Index` 0)
  (set `self.Face Montage Index` 0)
  (set `self.Sound Index` 0)
  (return))

(fn `Set Answer Size`
  (params (`New Scale` :type "Float (double-precision)"))
  (bind _answerwidgets (`self.AnswerWidgets`))
  (if (`KismetArrayLibrary.Array_IsValidIndex` _answerwidgets)
    (for _array_element _answerwidgets
      (`ScaleBox.SetUserSpecifiedScale` (`/Game/VRSubtitle/Widgets/WBP_AnAnswerWidget.ScaleBox_1` _array_element) `New Scale`)))
  (return))

(fn `Set Subtitle Size`
  (params (`New Scale` :type "Float (double-precision)"))
  (bind _dialoguewidgetref (`self.DialogueWidgetRef`)
    (:`then`
      (`ScaleBox.SetUserSpecifiedScale` (`/Game/VRSubtitle/Widgets/WBP_Subtitle.ScaleBox_0` _dialoguewidgetref) `New Scale`))
    (:`else`
      _))
  (return))

(fn `Show Error Message`
  (params (Message :type String))
  (for _ (range 3)
    (`KismetSystemLibrary.PrintString` Message true true (struct :`R` 1.0 :`G` 0.021699 :`A` 1.0) 15.0))
  (return))